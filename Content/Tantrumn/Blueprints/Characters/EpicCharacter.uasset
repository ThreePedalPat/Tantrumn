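; EpicCharacter is a character Blueprint whose event graph only prints vertical velocity on landing as debug output.
; Its Hold macro tells a tap from a hold using a retriggerable delay and two gates that open on press.
; Release before the delay ends fires Tap, while a press outlasting it fires Held and blocks Tap.
; OnJumped is empty, and the jump start time assignment is disconnected.
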(event EventOnJumped)

(event EventOnLanded
  (params (Hit :type Hit%20Result%20Structure%20%28by%20ref%29))
  (Development|PrintString (Utilities|String|ToString(Float) (.z (Transformation|GetVelocity)))))

(fn ConstructionScript)